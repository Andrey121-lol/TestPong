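; Networked Pong-style ball actor that bounces between paddles and walls, tracks both goals' scores and updates the score widget.
; StartServer launches it after a delay, and overlaps route through server-to-multicast events.
; Paddle hits reverse X and randomize Y from paddle velocity, while walls flip Y.
; Goals reset and relaunch it until a count reaches five, then the session is destroyed and the menu opens.
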(event `self.ReceiveBeginPlay`
  (bind _returnvalue (`|CreateWidget` "/Game/Test/Widgets/WDBP_Score.WDBP_Score_C"))
  (bind _output_get (set `self.Ref_ScoreWd` _returnvalue))
  (`UserWidget.AddToViewport` _output_get 0))

(event `Key|SpaceBar`
  (params (Key :type "Key Structure"))
  (:`Pressed`
    (`/Engine/EditorBlueprintResources/StandardMacros.DoOnce` false)))

(event `StartServer`
  (`self.MultiCastStartServer`))

(event `MultiCastStartServer`
  (`KismetSystemLibrary.Delay` 5.0)
  (`PrimitiveComponent.SetPhysicsLinearVelocity` (`self.StaticMesh`) (-2000.0 0.0 0.0) false "None"))

(event `self.ReceiveActorBeginOverlap`
  (params (OtherActor :type "Actor Object Reference"))
  (`self.MoveOnServer` OtherActor))

(event `MoveOnServer`
  (params (InputPin :type "Actor Object Reference"))
  (`self.MoveMultiCast` InputPin))

(event `MoveMultiCast`
  (params (InputPin :type "Actor Object Reference"))
  (bind _staticmesh (`self.StaticMesh`))
  (bind _staticmesh_2 (`self.StaticMesh`))
  (bind _staticmesh_3 (`self.StaticMesh`))
  (bind _staticmesh_4 (`self.StaticMesh`))
  (bind _ref_scorewd (`self.Ref_ScoreWd`))
  (bind _staticmesh_5 (`self.StaticMesh`))
  (bind _gameover (`self.GameOver`))
  (bind _asbp_apawn (cast `/Game/Test/BP/BP_Apawn` InputPin)
    (:`then`
      (bind _returnvalue (`PrimitiveComponent.GetPhysicsLinearVelocity` (`/Game/Test/BP/BP_Apawn.Platforma` _asbp_apawn) "None"))
      (bind _returnvalue_2 (`PrimitiveComponent.GetPhysicsLinearVelocity` _staticmesh_3 "None"))
      (`PrimitiveComponent.SetPhysicsLinearVelocity` _staticmesh_3 (`KismetMathLibrary.MakeVector` (* (.x _returnvalue_2) -1.0) (+ (.y _returnvalue) (`KismetMathLibrary.RandomFloatInRange` -3000.0 3000.0)) (.z _returnvalue_2)) false "None"))
    (:`CastFailed`
      (bind _asbp_enamy (cast `/Game/Test/BP/BP_Enamy` InputPin)
        (:`then`
          (bind _returnvalue_3 (`PrimitiveComponent.GetPhysicsLinearVelocity` (`/Game/Test/BP/BP_Enamy.StaticMesh` _asbp_enamy) "None"))
          (bind _returnvalue_4 (`PrimitiveComponent.GetPhysicsLinearVelocity` _staticmesh_4 "None"))
          (`PrimitiveComponent.SetPhysicsLinearVelocity` _staticmesh_4 (`KismetMathLibrary.MakeVector` (* (.x _returnvalue_4) -1.0) (+ (.y _returnvalue_3) (`KismetMathLibrary.RandomFloatInRange` -3000.0 3000.0)) (.z _returnvalue_4)) false "None"))
        (:`CastFailed`
          (cast `/Game/Test/BP/BP_Wall` InputPin
            (:`then`
              (bind _returnvalue_5 (`PrimitiveComponent.GetPhysicsLinearVelocity` _staticmesh_2 "None"))
              (`PrimitiveComponent.SetPhysicsLinearVelocity` _staticmesh_2 (`KismetMathLibrary.MakeVector` (.x _returnvalue_5) (* (.y _returnvalue_5) -1.0) (.z _returnvalue_5)) false "None"))
            (:`CastFailed`
              (cast `/Game/Test/BP/BP_Goal_L` InputPin
                (:`then`
                  (if _gameover
                    (`KismetSystemLibrary.PrintString` "Right win")
                    (else
                      (`PrimitiveComponent.SetPhysicsLinearVelocity` _staticmesh_5 (0.0 0.0 0.0) false "None")
                      (`self.K2_SetActorLocation` (0.0 0.0 90.0))
                      (bind _result (`/Engine/EditorBlueprintResources/StandardMacros.IncrementInt` (`self.LPlayer`))
                        (:`  `
                          (bind _output_get (set `self.LPlayer` _result))
                          (set `/Game/Test/Widgets/WDBP_Score.L_Score` _output_get _ref_scorewd)
                          (`KismetSystemLibrary.PrintString` (`KismetStringLibrary.Conv_IntToString` _output_get))
                          (if (> (`self.LPlayer`) 4)
                            (set `self.GameOver` true :!label _label)
                            (`DestroySessionCallbackProxy.DestroySession` (`GameplayStatics.GetPlayerController` 0)
                              (:`then`
                                (`GameplayStatics.OpenLevel` "menu")))
                            (else
                              (`KismetSystemLibrary.Delay` 1.0)
                              (`PrimitiveComponent.SetPhysicsLinearVelocity` _staticmesh (2000.0 0.0 0.0) false "None"))))))))
                (:`CastFailed`
                  (cast `/Game/Test/BP/BP_Goal_R` InputPin)
                  (if _gameover
                    (`KismetSystemLibrary.PrintString` "Left win")
                    (else
                      (`PrimitiveComponent.SetPhysicsLinearVelocity` _staticmesh_5 (0.0 0.0 0.0) false "None")
                      (`self.K2_SetActorLocation` (0.0 0.0 90.0))
                      (bind _result_2 (`/Engine/EditorBlueprintResources/StandardMacros.IncrementInt` (`self.RPlayer`))
                        (:`  `
                          (bind _output_get_2 (set `self.RPlayer` _result_2))
                          (set `/Game/Test/Widgets/WDBP_Score.R_Score` _output_get_2 _ref_scorewd)
                          (`KismetSystemLibrary.PrintString` (`KismetStringLibrary.Conv_IntToString` _output_get_2))
                          (if (> (`self.RPlayer`) 4)
                            (goto _label)
                            (else
                              (`KismetSystemLibrary.Delay` 1.0)
                              (`PrimitiveComponent.SetPhysicsLinearVelocity` _staticmesh (-2000.0 0.0 0.0) false "None"))))))))))))))))

(event `self.ReceiveTick`
  (params (DeltaSeconds :type "Float (single-precision)"))
  (bind _staticmesh (`self.StaticMesh`))
  (bind _returnvalue (`SceneComponent.K2_GetComponentLocation` _staticmesh))
  (`KismetSystemLibrary.LineTraceSingle` :`Start` _returnvalue :`End` (+ _returnvalue (* (`SceneComponent.GetForwardVector` _staticmesh) 100.0)) :`TraceChannel` "TraceTypeQuery1" :`DrawDebugType` "ForDuration"))

(fn `UserConstructionScript`)