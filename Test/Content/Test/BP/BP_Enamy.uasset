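; BP_Enamy is an AI-controlled physics actor that chases BP_ABall actors along the Y axis, apparently as an opponent paddle.
; Every Tick it finds all balls with GetAllActorsOfClass and calls MoveAi for each.
; MoveAi applies a Y impulse from the clamped ball offset scaled by AISpeed.
; Outside the fixed Y bounds, it instead snaps back to the limit and zeroes velocity.
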(event `self.ReceiveBeginPlay`)

(event `self.ReceiveTick`
  (params (DeltaSeconds :type "Float (single-precision)"))
  (bind _outactors (`GameplayStatics.GetAllActorsOfClass` "/Game/Test/BP/BP_ABall.BP_ABall_C"))
  (for _array_element _outactors
    (bind _asbp_aball (cast `/Game/Test/BP/BP_ABall` _array_element))
    (`self.MoveAi` _asbp_aball)))

(event `self.ReceiveActorBeginOverlap`
  (params (OtherActor :type "Actor Object Reference")))

(fn `MoveAi`
  (params (self2 :type "Actor Object Reference"))
  (if (> (.y (`self.K2_GetActorLocation`)) 1000.0)
    (`self.K2_SetActorLocation` (`KismetMathLibrary.MakeVector` (.x (`self.K2_GetActorLocation`)) 1000.0 (.z (`self.K2_GetActorLocation`))))
    (`PrimitiveComponent.SetPhysicsLinearVelocity` (0.0 0.0 0.0))
    (elif (< (.y (`self.K2_GetActorLocation`)) -1000.0)
      (`self.K2_SetActorLocation` (`KismetMathLibrary.MakeVector` (.x (`self.K2_GetActorLocation`)) -1000.0 (.z (`self.K2_GetActorLocation`))))
      (`PrimitiveComponent.SetPhysicsLinearVelocity` (0.0 0.0 0.0))
      (else
        (`PrimitiveComponent.AddImpulse` (* (`KismetMathLibrary.MakeVector` 0.0 (`KismetMathLibrary.FClamp` (- (.y (`self.K2_GetActorLocation` self2)) (.y (`self.K2_GetActorLocation`))) -10.0 10.0)) (`self.AI_Speed`)))))))

(fn `UserConstructionScript`)