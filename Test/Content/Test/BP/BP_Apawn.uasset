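; BP_Apawn is a test pawn that slides its Platforma component sideways from the RightMouseMove input axis.
; The axis value passes through MoveOnServer to MoveMultiCast, named as a server-then-multicast chain, which applies an inverted, Speed-scaled local X offset.
; If world Y is already beyond ±999, it snaps back to that limit instead of moving.
; BeginPlay calls AddWidgetServer, which is empty.
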(event `self.ReceiveBeginPlay`
  (`self.AddWidgetServer`))

(event `InputAxis|RightMouseMove`
  (params (AxisValue :type "Float (single-precision)"))
  (`self.MoveOnServer` AxisValue))

(event `MoveOnServer`
  (params (InputPin :type "Float (double-precision)"))
  (`self.MoveMultiCast` InputPin))

(event `MoveMultiCast`
  (params (InputPin :type "Float (double-precision)"))
  (bind _platforma (`self.Platforma`))
  (bind (_returnvalue_x _returnvalue_y _returnvalue_z) (`KismetMathLibrary.BreakVector` (`SceneComponent.K2_GetComponentLocation` _platforma)))
  (bind (_returnvalue_x_2 _returnvalue_y_2) (`KismetMathLibrary.BreakVector` (`SceneComponent.K2_GetComponentLocation` (`self.Platforma`))))
  (bind _returnvalue (> _returnvalue_y_2 999.0))
  (bind _returnvalue_2 (< _returnvalue_y_2 -999.0))
  (if (or _returnvalue _returnvalue_2)
    (if _returnvalue
      (`SceneComponent.K2_SetWorldLocation` _platforma (`KismetMathLibrary.MakeVector` _returnvalue_x 999.0 _returnvalue_z) false false)
      (elif _returnvalue_2
        (`SceneComponent.K2_SetWorldLocation` _platforma (`KismetMathLibrary.MakeVector` _returnvalue_x -999.0 _returnvalue_z) false false)))
    (else
      (`SceneComponent.K2_AddLocalOffset` (`self.Platforma`) (`KismetMathLibrary.MakeVector` (* (* InputPin -1.0) (`self.Speed`))) false false))))

(event `AddWidgetServer`)

(fn `UserConstructionScript`)